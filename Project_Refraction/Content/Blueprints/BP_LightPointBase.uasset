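; Base actor for a light point that fires a single forward trace shortly after play begins, apparently an early test of a light beam.
; After a short delay, ShootLight runs a Visibility line trace along the Arrow component's forward vector, draws it persistently and prints the hit actor's name.
; The actor adds itself to ActorsToIgnore, but the trace never uses that array.
; An alternative component trace on the Cone is left disconnected.
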(event `self.ReceiveBeginPlay`
  (`KismetArrayLibrary.Array_Add` (`self.Actors to Ignore`) self)
  (`KismetSystemLibrary.Delay` 2.5)
  (`self.ShootLight`))

(event `ShootLight`
  (bind _arrow (`self.Arrow`))
  (bind _returnvalue (`SceneComponent.K2_GetComponentLocation` _arrow))
  (bind _outhit (`KismetSystemLibrary.LineTraceSingle` :`Start` _returnvalue :`End` (+ (* (`KismetMathLibrary.GetForwardVector` (`SceneComponent.K2_GetComponentRotation` _arrow)) (`KismetMathLibrary.Conv_DoubleToVector` 5000.0)) _returnvalue) :`TraceChannel` "TraceTypeQuery1" :`DrawDebugType` "Persistent"))
  (`KismetSystemLibrary.PrintString` (`KismetSystemLibrary.GetDisplayName` (`.HitActor` (`GameplayStatics.BreakHitResult` _outhit)))))

(fn `UserConstructionScript`)